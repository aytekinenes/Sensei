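; Gameplay ability for a sword light attack that plays a replicated attack montage on the avatar once committed.
; It applies an attack gameplay effect to the owner and ends after a short delay.
; Midway, a debug-drawn forward multi-sphere trace gathers unique pawns in front of the avatar.
; Each hit pawn's ability system then activates abilities tagged React.Sword, so targets play their own reaction.
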(event Ability|EventActivateAbility
  (bind _returnvalue (Ability|CommitAbility))
  (if _returnvalue
    (Class|BPICharacter|PlayMontageReplicated(Message) (Ability|GetAvatarActorfromActorInfo) "/Game/SpearAnimationsV2/Animations/Character/2Hand/Pose03/EnesAnimation/AM_LightAttakc2.AM_LightAttakc2" 1.0 "None")
    (Utilities|FlowControl|Sequence
      (:then_0
        (Ability|ApplyGameplayEffectToOwner "/Game/BP/Abilities/GE_Attack.GE_Attack_C")
        (Utilities|FlowControl|Delay 0.2)
        (Ability|EndAbility))
      (:then_1
        (Utilities|FlowControl|Delay 0.1)
        (bind _hitactors1 (CallFunction|GetNearbyActors 8e+01))
        (for _array_element _hitactors1
          (Abilities|TryActivateAbilitiesbyTag (Ability|GetAbilitySystemComponent _array_element) (GameplayTags|MakeLiteralGameplayTagContainer "(GameplayTags=((TagName=\"React.Sword\")))") true))))))

(event Ability|EventOnEndAbility
  (params (bWasCancelled :type Boolean)))

(fn GetNearbyActors
  (params (Radius :type Float%20%28single-precision%29))
  (bind _returnvalue (Ability|GetAvatarActorfromActorInfo))
  (bind _returnvalue_2 (Transformation|GetActorLocation _returnvalue))
  (bind _returnvalue_3 (Transformation|GetActorForwardVector _returnvalue))
  (bind (_outhits _returnvalue_4) (Collision|MultiSphereTraceForObjects (+ _returnvalue_2 (* _returnvalue_3 5e+01)) (+ _returnvalue_2 (* _returnvalue_3 1e+02)) Radius (Utilities|Array|MakeArray "ObjectTypeQuery3") false 0 "ForDuration"))
  (if _returnvalue_4
    (for _array_element _outhits
      (Utilities|Array|AddUnique (LocalVariables|GetHitActors) (.HitActor (Collision|BreakHitResult _array_element))))
    (return (LocalVariables|GetHitActors))))